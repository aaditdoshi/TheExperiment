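; Blueprint actor for a room that appears in and disappears from the level by moving itself between a connected and a disconnected location.
; The construction script caches a self reference and two transforms, built from those locations with the actor's current rotation and unit scale, in MLevelDestination.
; MoveObjectToLevel and MoveObjectOutOfLevel call MakeRoomAppear and MakeRoomDisappear, which snap the actor to the attached or detached transform without sweeping.
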(event Custom|MoveObjectToLevel
  (CallFunction|MakeRoomAppear))

(event Custom|MoveObjectOutOfLevel
  (CallFunction|MakeRoomDisappear))

(event EventBeginPlay)

(event Collision|EventActorBeginOverlap
  (params (OtherActor :type Actor%20Object%20Reference)))

(event EventTick
  (params (DeltaSeconds :type Float%20%28single-precision%29)))

(fn ConstructionScript
  (bind _returnvalue (Transformation|GetActorRotation))
  (Variables|Default|SetmLevelDestination (Utilities|Struct|MakeLevelDestinations self (Math|Transform|MakeTransform (Variables|Default|GetConnectedLocation) _returnvalue) (Math|Transform|MakeTransform (Variables|Default|GetDisconnectedLocation) _returnvalue))))

(fn MakeRoomDisappear
  (bind _mleveldestination (Variables|Default|GetmLevelDestination))
  (Transformation|SetActorTransform (.mroom _mleveldestination) (.mdeteachedtransform _mleveldestination)))

(fn MakeRoomAppear
  (bind _mleveldestination (Variables|Default|GetmLevelDestination))
  (Transformation|SetActorTransform (.mroom _mleveldestination) (.mattachedtransform _mleveldestination)))